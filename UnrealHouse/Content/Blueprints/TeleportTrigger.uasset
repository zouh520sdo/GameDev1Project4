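; TeleportTrigger is a trigger actor that moves any overlapping actor to the transform of its Location actor reference.
; On overlap it creates a FadeInOutSeq level sequence player and calls PlayReverse then Play back to back, with no delay before the teleport.
; It also sets the first player controller's control rotation to Location's rotation, regardless of which actor overlapped.
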(event `self.ReceiveActorBeginOverlap`
  (params (OtherActor :type "Actor Object Reference"))
  (bind _location (`self.Location`))
  (bind _returnvalue (`self.K2_GetActorRotation` _location))
  (bind _outactor (`LevelSequencePlayer.CreateLevelSequencePlayer` "/Game/CameraSequences/FadeInOutSeq.FadeInOutSeq"))
  (bind _sequenceplayer (`LevelSequenceActor.SequencePlayer` _outactor))
  (`MovieSceneSequencePlayer.PlayReverse` _sequenceplayer)
  (`MovieSceneSequencePlayer.Play` _sequenceplayer)
  (`self.K2_SetActorTransform` OtherActor (`self.GetTransform` _location) false false)
  (`self.K2_SetActorRotation` OtherActor _returnvalue false)
  (`Controller.SetControlRotation` (`GameplayStatics.GetPlayerController` 0) _returnvalue))

(fn `UserConstructionScript`)