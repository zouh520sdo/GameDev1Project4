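; Bookshelf actor that swings open around its yaw axis when the player character stands inside its trigger volume.
; Tick polls the trigger overlap and plays a timeline whose Rotation track sets the mesh's relative yaw, with no reverse path.
; While the timeline updates, the audio component plays a random sound from an array whenever it is idle.
; BeginPlay enables player input, though no input events are bound.
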(event `self.ReceiveBeginPlay`
  (`self.EnableInput` (`GameplayStatics.GetPlayerController` 0)))

(event `self.ReceiveTick`
  (params (DeltaSeconds :type "Float (single-precision)"))
  (bind _soundarray (`self.SoundArray`))
  (bind _audio (`self.Audio`))
  (if (`self.IsOverlappingActor` (`self.TriggerVolume`) (`GameplayStatics.GetPlayerCharacter` 0))
    (bind (_direction _rotation) (`Timeline|Timeline_0`)
      (:`Update`
        (`SceneComponent.K2_SetRelativeRotation` (`self.StaticMeshComponent`) (`KismetMathLibrary.MakeRotator` 0.0 0.0 _rotation) false false)
        (if (not (`AudioComponent.IsPlaying` (`self.Audio`)))
          (`AudioComponent.SetSound` _audio (`|GetArrayItem` _soundarray (`KismetMathLibrary.RandomIntegerInRange` 0 (- (`KismetArrayLibrary.Array_Length` _soundarray) 1))))
          (`AudioComponent.Play` _audio 0.0))))))

(fn `UserConstructionScript`)