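; Phone actor that starts playing its audio on BeginPlay and can be answered by the player with the Space Bar.
; It enables input for the first player controller and accepts the key press only while the player character overlaps its Box.
; Answering stops the audio, makes every PointLight in the level visible and sets the referenced Door to zero rotation, repeating the Door call inside the light loop.
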(event `self.ReceiveBeginPlay`
  (`self.EnableInput` (`GameplayStatics.GetPlayerController` 0))
  (`AudioComponent.Play` (`self.Audio`) 0.0))

(event `Key|SpaceBar`
  (params (Key :type "Key Structure"))
  (:`Pressed`
    (if (`PrimitiveComponent.IsOverlappingActor` (`self.Box`) (`GameplayStatics.GetPlayerCharacter` 0))
      (`AudioComponent.Stop` (`self.Audio`))
      (bind _outactors (`GameplayStatics.GetAllActorsOfClass` "/Script/Engine.PointLight"))
      (for _array_element _outactors
        (`SceneComponent.SetVisibility` (`PointLight.PointLightComponent` _array_element) true false)
        (`self.K2_SetActorRotation` :`self` (`self.Door`))))))

(fn `UserConstructionScript`)