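; Bookshelf actor that moves and turns when the player character is inside its trigger volume.
; Tick polls the volume for overlap and plays a timeline that drives the mesh's relative location and yaw.
; The location track is added to the actor's world location before being set as a relative location.
; Input is enabled on BeginPlay, and random-sound playback logic exists but is never run.
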(event `self.ReceiveBeginPlay`
  (`self.EnableInput` (`GameplayStatics.GetPlayerController` 0)))

(event `self.ReceiveTick`
  (params (DeltaSeconds :type "Float (single-precision)"))
  (if (`self.IsOverlappingActor` (`self.TriggerVolume`) (`GameplayStatics.GetPlayerCharacter` 0))
    (bind (_direction _rotation _newtrack_1) (`Timeline|Timeline_0`)
      (:`Update`
        (`SceneComponent.K2_SetRelativeLocationAndRotation` (`self.StaticMeshComponent`) (+ _newtrack_1 (`self.K2_GetActorLocation`)) (`KismetMathLibrary.MakeRotator` 0.0 0.0 _rotation) false false)))))

(fn `UserConstructionScript`)